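; Dice actor that picks which tile type the player gets each round and counts it in the GlovalVars game instance.
; On BeginPlay it adds the dice UI widget and enables input; Space rolls only when the Placed flag is set, then clears it.
; A roll increments Round and re-randomizes until the value differs from the previous one.
; The result snaps the actor to that face's rotation, sets LatestType and increments that type's counter.
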(event `self.ReceiveBeginPlay`
  ;[1 1 1] Konstruktor
  (bind _returnvalue (`|CreateWidget` "/Game/GameObjects/Components/HUD/Dice_UI_widget.Dice_UI_widget_C"))
  (`UserWidget.AddToViewport` _returnvalue 0)
  (bind _asgloval_vars (cast `/Game/GameObjects/Components/Data/GlovalVars` (`GameplayStatics.GetGameInstance`)))
  (set `self.GlobalVarsRef` _asgloval_vars)
  (`self.EnableInput` (`GameplayStatics.GetPlayerController` 0)))

(event `Key|SpaceBar`
  (params (Key :type "Key Structure"))
  (bind _globalvarsref (`self.GlobalVarsRef`))
  ;[1 1 1] Kliknutie na blok
  (:`Pressed`
    (if (`/Game/GameObjects/Components/Data/GlovalVars.placed` _globalvarsref)
      (set `/Game/GameObjects/Components/Data/GlovalVars.placed` false _globalvarsref)
      (`self.Roll Dice`))))

(event `Roll Dice`
  ;[1 1 1] Comment
  (`/Engine/EditorBlueprintResources/StandardMacros.IncrementInt` (`/Game/GameObjects/Components/Data/GlovalVars.Round` (`self.GlobalVarsRef`))
    (:`  `
      (while (== (`self.Current`) (`self.LastVar`))
        (bind _roll (`self.RollDice`))
        (set `self.Current` _roll))
      (set `self.LastVar` (`self.Current`))
      (switch `/Game/GameObjects/Components/Enums/DiceNumber` (cast `/Game/GameObjects/Components/Enums/DiceNumber` (`KismetMathLibrary.Conv_IntToByte` (`self.Current`)))
        (:`NewEnumerator0`
          (`self.K2_SetActorTransform` (`KismetMathLibrary.MakeTransform` (`self.K2_GetActorLocation`) (`KismetMathLibrary.MakeRotator` 0.0)))
          (`self.AddCount` "NewEnumerator5"))
        (:`NewEnumerator1`
          (`self.K2_SetActorTransform` (`KismetMathLibrary.MakeTransform` (`self.K2_GetActorLocation`) (`KismetMathLibrary.MakeRotator` 0.0 180.0)))
          (`self.AddCount` "NewEnumerator1"))
        (:`NewEnumerator2`
          (`self.K2_SetActorTransform` (`KismetMathLibrary.MakeTransform` (`self.K2_GetActorLocation`) (`KismetMathLibrary.MakeRotator` 0.0 -90.0)))
          (`self.AddCount` "NewEnumerator4"))
        (:`NewEnumerator3`
          (`self.K2_SetActorTransform` (`KismetMathLibrary.MakeTransform` (`self.K2_GetActorLocation`) (`KismetMathLibrary.MakeRotator` 90.0)))
          (`self.AddCount` "NewEnumerator6"))
        (:`NewEnumerator4`
          (`self.K2_SetActorTransform` (`KismetMathLibrary.MakeTransform` (`self.K2_GetActorLocation`) (`KismetMathLibrary.MakeRotator` -90.0)))
          (`self.AddCount` "NewEnumerator8"))
        (:`NewEnumerator5`
          (`self.K2_SetActorTransform` (`KismetMathLibrary.MakeTransform` (`self.K2_GetActorLocation`) (`KismetMathLibrary.MakeRotator` 0.0 90.0)))
          (`self.AddCount` "NewEnumerator7"))))))

(fn `AddCount`
  (params (type :type "/Game/GameObjects/Components/Enums/BlocksEnums Enum" :default "NewEnumerator0"))
  (bind _globalvarsref (`self.GlobalVarsRef`))
  (set `/Game/GameObjects/Components/Data/GlovalVars.LatestType` type (`self.GlobalVarsRef`))
  (switch `/Game/GameObjects/Components/Enums/BlocksEnums` type
    (:`NewEnumerator1`
      (`/Engine/EditorBlueprintResources/StandardMacros.IncrementInt` (`/Game/GameObjects/Components/Data/GlovalVars.Pubs` _globalvarsref)))
    (:`NewEnumerator4`
      (`/Engine/EditorBlueprintResources/StandardMacros.IncrementInt` (`/Game/GameObjects/Components/Data/GlovalVars.Trees` _globalvarsref)))
    (:`NewEnumerator5`
      (`/Engine/EditorBlueprintResources/StandardMacros.IncrementInt` (`/Game/GameObjects/Components/Data/GlovalVars.Houses` _globalvarsref)))
    (:`NewEnumerator6`
      (`/Engine/EditorBlueprintResources/StandardMacros.IncrementInt` (`/Game/GameObjects/Components/Data/GlovalVars.Food` _globalvarsref)))
    (:`NewEnumerator7`
      (`/Engine/EditorBlueprintResources/StandardMacros.IncrementInt` (`/Game/GameObjects/Components/Data/GlovalVars.Wasteland` _globalvarsref)))
    (:`NewEnumerator8`
      (`/Engine/EditorBlueprintResources/StandardMacros.IncrementInt` (`/Game/GameObjects/Components/Data/GlovalVars.Water` _globalvarsref)))))

(fn `RollDice`
  (returns (roll :type Integer))
  (return (`KismetMathLibrary.RandomIntegerInRange` 0 5)))

(fn `UserConstructionScript`)