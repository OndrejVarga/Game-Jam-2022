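; SideBlock is a grid tile actor for a tile-placement builder, serving as a hidden candidate slot until clicked into a typed block such as house, pub, field or forest.
; Hovering previews the game instance's latest type, tinted red or green by whether a placement was already made.
; Clicking locks it in, restarts the game if house-to-food or house-to-pub balance fails, then spawns unoccupied four-way neighbours, registered in a global grid array.
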(event `self.ReceiveBeginPlay`
  ;[1 1 1] Konstruktor
  (bind _asgloval_vars (cast `/Game/GameObjects/Components/Data/GlovalVars` (`GameplayStatics.GetGameInstance`)))
  (set `self.Global vars ref` _asgloval_vars)
  (`self.SetActorHiddenInGame` true)
  (add `self.OnBeginCursorOver` (delegate `CustomEvent`))
  (add `self.OnEndCursorOver` (delegate `CustomEvent_1`))
  (add `self.OnClicked` (delegate `CustomEvent_2`)))

(event `CustomEvent` :!signature `self.OnBeginCursorOver`
  (params (TouchedActor :type "Actor Object Reference"))
  (bind _global_vars_ref (`self.Global vars ref`))
  ;[1 1 1] Mouse Hober start
  (if (`self.Is Active`)
    _
    (elif (not (`self.Highlighted?`))
      (`self.Set Type` (`/Game/GameObjects/Components/Data/GlovalVars.LatestType` _global_vars_ref))
      (if (`/Game/GameObjects/Components/Data/GlovalVars.placed` _global_vars_ref)
        (`PrimitiveComponent.SetMaterial` (`self.SideBlock`) 0 "/Game/GameObjects/Materials/RedMaterial.RedMaterial")
        (set `self.Highlighted?` true)
        (`self.SetActorHiddenInGame` false)
        (else
          (`PrimitiveComponent.SetMaterial` (`self.SideBlock`) 0 "/Game/GameObjects/Materials/GreenMaterial.GreenMaterial")
          (set `self.Highlighted?` true)
          (`self.SetActorHiddenInGame` false))))))

(event `CustomEvent_1` :!signature `self.OnEndCursorOver`
  (params (TouchedActor :type "Actor Object Reference"))
  ;[1 1 1] Mouse Hover end
  (if (`self.Is Active`)
    _
    (elif (`self.Highlighted?`)
      (set `self.Highlighted?` false)
      (`self.SetActorHiddenInGame` true))))

(event `Set Type`
  (params (BlockType :type "/Game/GameObjects/Components/Enums/BlocksEnums Enum" :default "NewEnumerator0"))
  (bind _sideblock (`self.SideBlock`))
  (bind _sideblock_2 (`self.SideBlock`))
  ;[1 1 1] Setting Mesh
  (bind _output_get (set `self.type` BlockType))
  (switch `/Game/GameObjects/Components/Enums/BlocksEnums` _output_get
    (:`NewEnumerator0`
      (`PrimitiveComponent.SetMaterial` (`self.SideBlock`) 0 "/Game/GameObjects/Materials/GreenMaterial.GreenMaterial")
      (`StaticMeshComponent.SetStaticMesh` (`self.SideBlock`) "/Game/GameObjects/Models/bloky/Pustatina.Pustatina"))
    (:`NewEnumerator1`
      (`PrimitiveComponent.SetMaterial` (`self.SideBlock`) 0 "/Game/GameObjects/Materials/Blocks/krcma_material.krcma_material")
      (`PrimitiveComponent.SetMaterial` (`self.SideBlock`) 1 "/Game/GameObjects/Materials/Blocks/krcma_dom_material.krcma_dom_material")
      (`StaticMeshComponent.SetStaticMesh` (`self.SideBlock`) "/Game/GameObjects/Models/bloky/krcma.krcma"))
    (:`NewEnumerator4`
      (`PrimitiveComponent.SetMaterial` _sideblock 0 "/Game/GameObjects/Materials/Blocks/les_material.les_material")
      (`PrimitiveComponent.SetMaterial` _sideblock 1 "/Game/GameObjects/Materials/Blocks/strom3_material.strom3_material")
      (`PrimitiveComponent.SetMaterial` _sideblock 2 "/Game/GameObjects/Materials/Blocks/strom2_material.strom2_material")
      (`PrimitiveComponent.SetMaterial` _sideblock 3 "/Game/GameObjects/Materials/Blocks/strom1_material.strom1_material")
      (`StaticMeshComponent.SetStaticMesh` _sideblock "/Game/GameObjects/Models/bloky/Stromy.Stromy"))
    (:`NewEnumerator5`
      (`PrimitiveComponent.SetMaterial` (`self.SideBlock`) 0 "/Game/GameObjects/Materials/Blocks/dom_material.dom_material")
      (`PrimitiveComponent.SetMaterial` _sideblock_2 1 "/Game/GameObjects/Materials/Blocks/blok_dom_material.blok_dom_material")
      (`StaticMeshComponent.SetStaticMesh` _sideblock_2 "/Game/GameObjects/Models/bloky/Dom.Dom"))
    (:`NewEnumerator6`
      (`PrimitiveComponent.SetMaterial` (`self.SideBlock`) 1 "/Game/GameObjects/Materials/Blocks/pole_material.pole_material")
      (`PrimitiveComponent.SetMaterial` (`self.SideBlock`) 0 "/Game/GameObjects/Materials/Blocks/stohy_material.stohy_material")
      (`StaticMeshComponent.SetStaticMesh` (`self.SideBlock`) "/Game/GameObjects/Models/bloky/Pole.Pole"))
    (:`NewEnumerator7`
      (`PrimitiveComponent.SetMaterial` (`self.SideBlock`) 0 "/Game/GameObjects/Materials/Blocks/Pustatina.Pustatina")
      (`StaticMeshComponent.SetStaticMesh` (`self.SideBlock`) "/Game/GameObjects/Models/bloky/Pustatina.Pustatina"))
    (:`NewEnumerator8`
      (`PrimitiveComponent.SetMaterial` (`self.SideBlock`) 0 "/Game/GameObjects/Materials/GreenMaterial.GreenMaterial")
      (`StaticMeshComponent.SetStaticMesh` (`self.SideBlock`) "/Game/GameObjects/Models/bloky/Pustatina.Pustatina"))))

(event `CustomEvent_2` :!signature `self.OnClicked`
  (params (TouchedActor :type "Actor Object Reference") (ButtonPressed :type "Key Structure" :default "None"))
  ;[1 1 1] Mouse event
  (if (not (`/Game/GameObjects/Components/Data/GlovalVars.placed` (`self.Global vars ref`)))
    (if (not (`self.Is Active`))
      (set `self.Is Active` true)
      (`self.Set Type` (`self.type`))
      (`self.CheckDead`)
      (`self.Create Neightbours`)
      (set `/Game/GameObjects/Components/Data/GlovalVars.placed` true (`self.Global vars ref`)))))

(event `Create Neightbours`
  (bind _returnvalue (`self.K2_GetActorLocation`))
  ;[1 1 1] Vytvori potencialne bloky v okoli tohto bloku
  (`self.CreateBlock` _returnvalue)
  (`self.CreateBlock` _returnvalue "NewEnumerator1")
  (`self.CreateBlock` _returnvalue "NewEnumerator3")
  (`self.CreateBlock` _returnvalue "NewEnumerator2"))

(event `CheckDead`
  (bind _global_vars_ref (`self.Global vars ref`))
  ;[1 1 1] Check for game end
  (if (not (and (> (- (`/Game/GameObjects/Components/Data/GlovalVars.Houses` _global_vars_ref) (`/Game/GameObjects/Components/Data/GlovalVars.Food` _global_vars_ref)) -5) (> (- (`/Game/GameObjects/Components/Data/GlovalVars.Houses` _global_vars_ref) (`/Game/GameObjects/Components/Data/GlovalVars.Pubs` _global_vars_ref)) -5)))
    (bind _asgame_mode (cast `GameMode` (`GameplayStatics.GetGameMode`)))
    (`GameMode.RestartGame` _asgame_mode)))

(fn `AddToArray`
  (params (SideBlock :type "/Game/GameObjects/Components/Blueprints/SideBlock Object Reference") (Location :type "Vector Structure"))
  (`KismetArrayLibrary.Array_Add` (`/Game/GameObjects/Components/Data/GlovalVars.GridArrayGlob` (`self.Global vars ref`)) (make `/Game/GameObjects/Components/Data/PlacedBlocksStruct` SideBlock Location)))

(fn `CreateBlock`
  (params (Location :type "Vector Structure") (Side :type "/Game/GameObjects/Components/Enums/SidesEnums Enum" :default "NewEnumerator0"))
  (returns (Object :type "/Game/GameObjects/Components/Blueprints/SideBlock Object Reference"))
  (bind _returnvalue (`KismetMathLibrary.MakeVector` (.x Location) (+ (.y Location) -200.0) (.z Location)))
  (bind _returnvalue_2 (`KismetMathLibrary.MakeVector` (+ (.x Location) 200.0) (.y Location) (.z Location)))
  (bind _returnvalue_3 (`KismetMathLibrary.MakeVector` (+ (.x Location) -200.0) (.y Location) (.z Location)))
  (bind _returnvalue_4 (`KismetMathLibrary.MakeVector` (.x Location) (+ (.y Location) 200.0) (.z Location)))
  ;[1 1 1] Funkcia, ktora vypocita poziciu a vytvari nove bloky hore, dole, vpravo a vlavo
  (switch `/Game/GameObjects/Components/Enums/SidesEnums` Side
    (:`NewEnumerator0`
      (bind _valid (`self.isValidToCreateBlock` _returnvalue_2))
      (if _valid
        (bind _returnvalue_5 (`|SpawnActorFromClass` "SideBlock_C" (`KismetMathLibrary.Conv_VectorToTransform` _returnvalue_2) "AlwaysSpawn" "OverrideRootScale" null null))
        (`self.AddToArray` _returnvalue_5 _returnvalue_2)
        (return _returnvalue_5)))
    (:`NewEnumerator1`
      (bind _valid_2 (`self.isValidToCreateBlock` _returnvalue_3))
      (if _valid_2
        (bind _returnvalue_6 (`|SpawnActorFromClass` "SideBlock_C" (`KismetMathLibrary.Conv_VectorToTransform` _returnvalue_3) "AlwaysSpawn" "OverrideRootScale" null null))
        (`self.AddToArray` _returnvalue_6 _returnvalue_3)
        (return _returnvalue_6)))
    (:`NewEnumerator2`
      (bind _valid_3 (`self.isValidToCreateBlock` _returnvalue_4))
      (if _valid_3
        (bind _returnvalue_7 (`|SpawnActorFromClass` "SideBlock_C" (`KismetMathLibrary.Conv_VectorToTransform` _returnvalue_4) "AlwaysSpawn" "OverrideRootScale" null null))
        (`self.AddToArray` null _returnvalue_4)
        (return _returnvalue_7)))
    (:`NewEnumerator3`
      (bind _valid_4 (`self.isValidToCreateBlock` _returnvalue))
      (if _valid_4
        (bind _returnvalue_8 (`|SpawnActorFromClass` "SideBlock_C" (`KismetMathLibrary.Conv_VectorToTransform` _returnvalue) "AlwaysSpawn" "OverrideRootScale" null null))
        (`self.AddToArray` _returnvalue_8 _returnvalue)
        (return _returnvalue_8)))))

(fn `isValidToCreateBlock`
  (params (Location :type "Vector Structure"))
  (returns (Valid :type Boolean))
  (for _array_element (`/Game/GameObjects/Components/Data/GlovalVars.GridArrayGlob` (`self.Global vars ref`))
    (if (== (`.Location_15_255BB0154B39724FC0CEA5ACCFB1F0B5` (break `/Game/GameObjects/Components/Data/PlacedBlocksStruct` _array_element)) Location)
      (return false)))
  (return true))

(fn `isValidToCreateBlock_0`
  (params (Location :type "Vector Structure"))
  (returns (Valid :type Boolean))
  (for _array_element (`/Game/GameObjects/Components/Data/GlovalVars.GridArrayGlob` (`self.Global vars ref`))
    (if (== Location (`.Location_15_255BB0154B39724FC0CEA5ACCFB1F0B5` (break `/Game/GameObjects/Components/Data/PlacedBlocksStruct` _array_element)))
      (return false)))
  (return true))

(fn `UserConstructionScript`)